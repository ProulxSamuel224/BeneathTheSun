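; BP_Corridor is a corridor actor that shows a crosshair marker while it is targeted.
; The targeted and untargeted events toggle TargetCrossair visibility, and BeginPlay disables the marker's shadow.
; An unconnected chain that never runs would move the crosshair to GetEnemySpawnLocation and spawn a BP_BaseEnemy there.
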(event `self.OnCorridorUnTargetted`
  (`SceneComponent.SetVisibility` (`self.TargetCrossair`) false false))

(event `self.OnCorridorTargetted`
  (`SceneComponent.SetVisibility` (`self.TargetCrossair`) true false))

(event `self.ReceiveBeginPlay`
  (`PrimitiveComponent.SetCastShadow` (`self.TargetCrossair`) false))

(fn `UserConstructionScript`)